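; Paintable wall that records paint hits from the VR pawn's line trace on a render target.
; Construction creates the wall render target plus dynamic materials for display, paint brush and heat splat; BeginPlay clears the target and binds it to the wall.
; paintHit converts hits to collision UVs, then draws brush materials into the wall target and a separate heatmap target.
; CLEARCANVAS wipes only the wall target.
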(event `CLEAR CANVAS`
  ;[1 1 1] CLEAR WALL EVENT
  (`KismetRenderingLibrary.ClearRenderTarget2D` (`self.wall_RT_ref`)))

(event `self.ReceiveBeginPlay`
  ;[1 1 1] EVENT BEGIN PLAY
  ;;[1 1 1] CLEAR WALL
  (`KismetRenderingLibrary.ClearRenderTarget2D` (`self.wall_RT_ref`))
  ;;[1 1 1] SET WALL MID TO RENDER TARGET
  (`MaterialInstanceDynamic.SetTextureParameterValue` (`self.wallMID_ref`) "RTtexture" (`self.wall_RT_ref`)))

(event `paintHit`
  (params (uvHit :type "HitResult Structure") (color :type "LinearColor Structure"))
  (bind _uv (`GameplayStatics.FindCollisionUV` uvHit))
  (bind _bg_brush_ref (`self.BG_Brush_ref`))
  (bind _returnvalue (`KismetMathLibrary.Conv_VectorToLinearColor` (`KismetMathLibrary.Conv_Vector2DToVector` _uv)))
  ;[1 1 1] PAINT HIT EVENTS. GETS CALLED FROM vrPAWN LINE TRACE
  ;;[1 1 1] CHECK IF COLOR IS SAME
  (if (not (`KismetStringLibrary.EqualEqual_StrStr` (`KismetStringLibrary.Conv_ColorToString` (`self.color`)) (`KismetStringLibrary.Conv_ColorToString` color)))
    ;;[1 1 1] IF NOT SAME COLOR SET PAINT MID COLOR
    (bind _output_get (set `self.color` color))
    (`MaterialInstanceDynamic.SetVectorParameterValue` (`self.paintMID_ref`) "Color" _output_get))
  ;;[1 1 1] UV HIT SET PAINT POSITION ON WALL
  (`MaterialInstanceDynamic.SetVectorParameterValue` (`self.paintMID_ref`) "ForcePosition" _returnvalue)
  (`KismetSystemLibrary.PrintString` (`KismetStringLibrary.Conv_ColorToString` _returnvalue) false false)
  ;;[1 1 1] DRAW ONTO RENDER TARGET
  (`KismetRenderingLibrary.DrawMaterialToRenderTarget` (`self.wall_RT_ref`) (`self.paintMID_ref`))
  (set `self.Heatmap_Location` _uv)
  ;[0.3416 0.4427 1] Draw to HeatMap
  (`MaterialInstanceDynamic.SetScalarParameterValue` _bg_brush_ref "Size" 0.02)
  ;;[1 1 1] Heatmap Strength
  (`MaterialInstanceDynamic.SetScalarParameterValue` _bg_brush_ref "Strength" 0.05)
  (`MaterialInstanceDynamic.SetVectorParameterValue` _bg_brush_ref "Position" (`KismetMathLibrary.Conv_VectorToLinearColor` (`KismetMathLibrary.Conv_Vector2DToVector` _uv)))
  (`KismetRenderingLibrary.DrawMaterialToRenderTarget` (`self.BG_RT_ref`) (`self.BG_Brush_ref`)))

(fn `UserConstructionScript`
  ;[1 1 1] CREATE RENDER TARGET AND DYNAMIC MATERIAL INSTANCES AND SET MATERIAL
  (bind _returnvalue (`KismetRenderingLibrary.CreateRenderTarget2D` (`self.RT_Width`) (`self.RT_Height`)))
  (set `self.wall_RT_ref` _returnvalue)
  (bind _returnvalue_2 (`KismetMaterialLibrary.CreateDynamicMaterialInstance` "/Game/Materials/wallRenderTarget_Mat.wallRenderTarget_Mat"))
  (bind _output_get (set `self.wallMID_ref` _returnvalue_2))
  (`PrimitiveComponent.SetMaterial` (`self.StaticMeshComponent`) 0 _output_get)
  (bind _returnvalue_3 (`KismetMaterialLibrary.CreateDynamicMaterialInstance` "/Game/Materials/paintMat.paintMat"))
  (set `self.paintMID_ref` _returnvalue_3)
  (bind _returnvalue_4 (`KismetMaterialLibrary.CreateDynamicMaterialInstance` "/Game/Models/M_HeatSplat.M_HeatSplat"))
  (set `self.BG_Brush_ref` _returnvalue_4)
  (set `self.container` (`self.Scene`)))
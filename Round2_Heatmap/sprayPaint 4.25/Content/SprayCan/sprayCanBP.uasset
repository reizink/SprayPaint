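; VR spray can that follows the first tracked SteamVR controller and paints on walls.
; While the right trigger is held, Tick runs a short complex line trace from the Arrow and passes hits to WallBP's PaintHit.
; Right thumbstick press raises SpraySize and sets the paint material's forceSize parameter; left grip 1 lowers only the variable.
; Other controller inputs, Space and BeginPlay only print debug text.
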(event `Key|MotionController_Right_Thumbstick`
  (params (Key :type "Key Structure" :default "AnyKey"))
  (:`Pressed`
    (if (not (>= (`self.spray_size`) 1.0))
      (bind _output_get (set `self.spray_size` (+ (`self.spray_size`) 0.01)))
      (`MaterialInstanceDynamic.SetScalarParameterValue` (`self.paintMID_ref`) "forceSize" _output_get)
      (`KismetSystemLibrary.PrintString` "RIGHT THUMBSTICK INCREASE SIZE"))))

(event `Key|MotionController_Left_Thumbstick`
  (params (Key :type "Key Structure" :default "AnyKey"))
  (:`Pressed`
    (`KismetSystemLibrary.PrintString` "LEFT THUMBSTICK INCREASE SIZE")))

(event `Key|MotionController_Left_Grip1`
  (params (Key :type "Key Structure" :default "AnyKey"))
  (:`Pressed`
    (if (not (`KismetMathLibrary.NearlyEqual_FloatFloat` (`self.spray_size`)))
      (set `self.spray_size` (- (`self.spray_size`) 0.01))
      (`KismetSystemLibrary.PrintString` "LEFT GRIP 1 DECREASE SIZE"))))

(event `Key|MotionController_Left_Grip2`
  (params (Key :type "Key Structure" :default "AnyKey"))
  (:`Pressed`
    (`KismetSystemLibrary.PrintString` "LEFT GRIP 2 DECREASE SIZE")))

(event `Key|MotionController_Right_Grip1`
  (params (Key :type "Key Structure" :default "AnyKey"))
  (:`Pressed`
    (`KismetSystemLibrary.PrintString` "RIGHT GRIP 1 DECREASE SIZE")))

(event `Key|MotionController_Right_Grip2`
  (params (Key :type "Key Structure" :default "AnyKey"))
  (:`Pressed`
    (`KismetSystemLibrary.PrintString` "RIGHT GRIP 2 DECREASE SIZE")))

(event `Key|MotionController_Left_Trigger`
  (params (Key :type "Key Structure" :default "AnyKey"))
  (:`Pressed`
    (`KismetSystemLibrary.PrintString` "LEFT TRIGGER"))
  (:`Released`
    (`KismetSystemLibrary.PrintString` "LEFT TRIGGER RELEASE")))

(event `Key|MotionController_Right_Trigger`
  (params (Key :type "Key Structure" :default "AnyKey"))
  (:`Pressed`
    (`KismetSystemLibrary.PrintString` "RIGHT TRIGGER")
    (set `self.spraying?` true))
  (:`Released`
    (`KismetSystemLibrary.PrintString` "RIGHT TRIGGER RELEASE")
    (set `self.spraying?` false)))

(event `Key|SpaceBar`
  (params (Key :type "Key Structure" :default "AnyKey"))
  (:`Pressed`
    (`KismetSystemLibrary.PrintString` (`KismetStringLibrary.Conv_IntToString` (`KismetArrayLibrary.Array_Length` (`SteamVRFunctionLibrary.GetValidTrackedDeviceIds` "Controller"))))
    (`KismetSystemLibrary.PrintString` (`|GetEnumeratorNameAsString` (`MotionControllerComponent.CurrentTrackingStatus` (`self.MotionController`))))))

(event `self.ReceiveBeginPlay`
  (bind _outactors (`GameplayStatics.GetAllActorsOfClass` "/Game/Wall/wallBP.wallBP_C"))
  (`KismetSystemLibrary.PrintString` (`KismetSystemLibrary.GetDisplayName` (`/Game/Wall/wallBP.paintMID_ref` (`KismetArrayLibrary.Array_Get` _outactors)))))

(event `self.ReceiveTick`
  (params (DeltaSeconds :type "Float (single-precision)"))
  (bind (_outposition _outorientation) (`SteamVRFunctionLibrary.GetTrackedDevicePositionAndOrientation` (`KismetArrayLibrary.Array_Get` (`SteamVRFunctionLibrary.GetValidTrackedDeviceIds` "Controller"))))
  (set `self.delta` DeltaSeconds)
  (`|ExecutionSequence`
    (:`then_0`
      (`SceneComponent.K2_SetWorldLocationAndRotation` (`self.Scene`) _outposition _outorientation false false))
    (:`then_1`
      (if (`self.spraying?`)
        (`self.LineTrace`)))))

(fn `LineTrace`
  (bind _arrow (`self.Arrow`))
  (bind _returnvalue (`SceneComponent.K2_GetComponentLocation` _arrow))
  (bind (_outhit _returnvalue_2) (`KismetSystemLibrary.LineTraceSingle` _returnvalue (+ _returnvalue (* (`KismetMathLibrary.GetForwardVector` (`SceneComponent.K2_GetComponentRotation` _arrow)) 350.0)) "TraceTypeQuery1" true))
  (if _returnvalue_2
    (bind (_bblockinghit _binitialoverlap _time _location _impactpoint _normal _impactnormal _physmat _hitactor) (`GameplayStatics.BreakHitResult` _outhit))
    (`/Engine/EditorBlueprintResources/StandardMacros.IsValid` _hitactor
      (:`Is Valid`
        (bind _aswall_bp (cast `/Game/Wall/wallBP` _hitactor))
        (`/Game/Wall/wallBP.paintHit` _aswall_bp _outhit)))))

(fn `UserConstructionScript`)
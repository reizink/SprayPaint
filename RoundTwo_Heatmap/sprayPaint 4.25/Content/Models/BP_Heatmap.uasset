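; Heatmap actor that the player paints onto by holding left mouse, with Space and BeginPlay clearing its render target to black.
; While spraying, Tick runs a debug-drawn multi line trace from PlayerRef along the control rotation, keeping blocking hits on this actor.
; Each hit is converted into PositionGatheringPlane's local space, scaled by Resolution, and drawn into the render target through a dynamic M_HeatSplat material as a small, low-strength splat.
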(event `Key|LeftMouseButton`
  (params (Key :type "Key Structure"))
  ;[1 1 1] Set Spray on Click
  (:`Pressed`
    (set `self.Spraying?` true))
  (:`Released`
    (set `self.Spraying?` false)))

(event `Key|SpaceBar`
  (params (Key :type "Key Structure"))
  ;[1 1 1] Clear Canvas with Space
  (:`Pressed`
    (`KismetRenderingLibrary.ClearRenderTarget2D` (`self.RenderTargetRuntime`))))

(event `self.ReceiveBeginPlay`
  ;[1 1 1] Clear Canvas at Beginning
  (`KismetRenderingLibrary.ClearRenderTarget2D` (`self.RenderTargetRuntime`)))

(event `self.ReceiveTick`
  (params (DeltaSeconds :type "Float (single-precision)"))
  (bind _player_ref (`self.Player_Ref`))
  (bind _returnvalue (`self.K2_GetActorLocation` _player_ref))
  ;[1 1 1] Event Tick: Trace Vector
  (`/Engine/EditorBlueprintResources/StandardMacros.IsValid` _player_ref
    (:`Is Valid`
      (if (`self.Spraying?`)
        (bind _outhits (`KismetSystemLibrary.LineTraceMultiForObjects` :`Start` _returnvalue :`End` (+ _returnvalue (* (`KismetMathLibrary.Conv_RotatorToVector` (`Pawn.GetControlRotation` _player_ref)) 1000.0)) :`ObjectTypes` (`|MakeArray` "ObjectTypeQuery1" "ObjectTypeQuery2" :!type "EObjectTypeQuery Enum") :`DrawDebugType` "ForOneFrame" :`bIgnoreSelf` false))
        (for _array_element _outhits
          (bind (_bblockinghit _binitialoverlap _time _distance _location _impactpoint _normal _impactnormal _physmat _hitactor) (`GameplayStatics.BreakHitResult` _array_element))
          (if (and _bblockinghit (== _hitactor self))
            (`self.DrawToRenderTarget` _location 0.01 0.03)))))))

(event `DrawToRenderTarget`
  (params (Location :type "Vector Structure") (Strength :type "Float (double-precision)") (Size :type "Float (double-precision)"))
  (bind _mid_heatsplat (`self.MID_HeatSplat`))
  ;[1 1 1] Draw to Render Target
  (`MaterialInstanceDynamic.SetScalarParameterValue` _mid_heatsplat "Size" Size)
  (`MaterialInstanceDynamic.SetScalarParameterValue` _mid_heatsplat "Strength" Strength)
  (`MaterialInstanceDynamic.SetVectorParameterValue` _mid_heatsplat "Position" (`KismetMathLibrary.Conv_VectorToLinearColor` (/ (`KismetMathLibrary.TransformLocation` (`KismetMathLibrary.InvertTransform` (`SceneComponent.K2_GetComponentToWorld` (`self.PositionGatheringPlane`))) Location) (`self.Resolution`))))
  (`KismetRenderingLibrary.DrawMaterialToRenderTarget` (`self.RenderTargetRuntime`) _mid_heatsplat))

(fn `UserConstructionScript`
  (bind _returnvalue (`KismetMaterialLibrary.CreateDynamicMaterialInstance` "/Game/Models/M_HeatSplat.M_HeatSplat"))
  (set `self.MID_HeatSplat` _returnvalue))
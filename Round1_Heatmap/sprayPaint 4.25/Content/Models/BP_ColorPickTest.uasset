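; BP_ColorPickTest is a test Blueprint that samples the color at the center of the RenderTarget_ColorPick render target.
; A looping timer started on BeginPlay repeatedly reads the pixel at half of XScreenSize and YScreenSize.
; Each sample is stored as both a Color and a LinearColor, and the linear value is printed as debug text.
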(event `self.ReceiveBeginPlay`
  (`KismetSystemLibrary.K2_SetTimerDelegate` (delegate `CP_Event`) 0.1 true))

(event `CP_Event`
  (bind _returnvalue (`KismetRenderingLibrary.ReadRenderTargetPixel` "/Game/Models/RenderTarget_ColorPick.RenderTarget_ColorPick" (/ (`self.X_ScreenSize`) 2) (/ (`self.Y_ScreenSize`) 2)))
  (bind _output_get (set `self.ColorSt_ref` _returnvalue))
  (bind _output_get_2 (set `self.ColorL_ref` (`KismetMathLibrary.Conv_ColorToLinearColor` _output_get)))
  (`KismetSystemLibrary.PrintString` (`KismetStringLibrary.Conv_ColorToString` _output_get_2)))

(fn `UserConstructionScript`)
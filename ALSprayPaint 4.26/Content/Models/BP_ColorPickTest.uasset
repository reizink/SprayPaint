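; BP_ColorPickTest is a test Blueprint that detects paint drips from a heatmap scene capture during spraying.
; A looping timer samples the center pixel of the color-pick render target and compares it to a red drip threshold.
; DripBool latches so each entry into red triggers only once, printing a debug message and raising the TellVRPawn flag until the next sample.
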(event `self.ReceiveBeginPlay`
  (`KismetSystemLibrary.K2_SetTimerDelegate` (delegate `CP_Event`) 0.1 true))

(event `CP_Event`
  (bind (_r _g _b) (break `LinearColor` (`self.DripLimit`)))
  ;[1 1 1] Get color of Heatmap - Center of Screen Capture rendering
  (bind _returnvalue (`KismetRenderingLibrary.ReadRenderTargetPixel` "/Game/Models/RenderTarget_ColorPick.RenderTarget_ColorPick" (/ (`self.X_ScreenSize`) 2) (/ (`self.Y_ScreenSize`) 2)))
  (bind _output_get (set `self.ColorSt_ref` _returnvalue))
  (bind _output_get_2 (set `self.ColorL_ref` (`KismetMathLibrary.Conv_ColorToLinearColor` _output_get)))
  ;[1 1 1] Is Heatmap above Drip Limit (RED)
  (set `self.TellVRPawn` false)
  (bind (_r_2 _g_2 _b_2) (break `LinearColor` _output_get_2))
  ;[1 1 1] Drip Once in Red Area While Spraying
  (if (and (>= _r_2 _r) (<= _g_2 _g) (<= _b_2 _b))
    (if (not (`self.DripBool`))
      (set `self.DripBool` true)
      (`KismetSystemLibrary.PrintString` "Drip: Red")
      (set `self.TellVRPawn` true))
    (else
      (set `self.DripBool` false))))

(fn `UserConstructionScript`)
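; Test Blueprint for a Niagara drip/spray effect that reports particle positions back to Blueprint.
; BeginPlay registers the actor as the system's BP_ParticleInfo object so it receives particle data callbacks.
; Each exported particle gets a visibility trace from the VrPawn's MiddlePos to its position, with positions and impact points only printed.
; Tick mirrors BP_ColorPickTest's TellVRPawn flag into User.Spraying, looking that actor up every frame.
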(event `self.ReceiveBeginPlay`
  ;[1 1 1] Particle Connect to BP
  (`NiagaraComponent.SetNiagaraVariableObject` (`self.Niagara`) "BP_ParticleInfo" self))

(event `self.ReceiveParticleData`
  (params (Data :type "Array of BasicParticleData Structure (by ref)") (NiagaraSystem :type "NiagaraSystem Object Reference"))
  ;[1 1 1] Get Particle Data, Print
  (`KismetSystemLibrary.PrintString` "PARTICLE DATA")
  (for _array_element Data
    (bind _position (break `BasicParticleData` _array_element))
    (`KismetSystemLibrary.PrintString` (`KismetStringLibrary.Conv_VectorToString` _position))
    (bind _outactors (`GameplayStatics.GetAllActorsOfClass` "/Game/SprayCan/Blueprints/vrPawn.vrPawn_C"))
    (bind _outhit (`KismetSystemLibrary.LineTraceSingle` (`/Game/SprayCan/Blueprints/vrPawn.MiddlePos` (`|GetArrayItem` _outactors)) _position "TraceTypeQuery1"))
    (`KismetSystemLibrary.PrintString` (`KismetStringLibrary.Conv_VectorToString` (`.ImpactPoint` (`GameplayStatics.BreakHitResult` _outhit))))))

(event `self.ReceiveTick`
  (params (DeltaSeconds :type "Float (single-precision)"))
  ;[1 1 1] Try Setting variable to get particle data (Works once)
  (set `self.Delta` DeltaSeconds)
  (bind _outactors (`GameplayStatics.GetAllActorsOfClass` "/Game/Models/BP_ColorPickTest.BP_ColorPickTest_C"))
  (if (`/Game/Models/BP_ColorPickTest.TellVRPawn` (`|GetArrayItem` _outactors))
    (`NiagaraComponent.SetVariableBool` (`self.Niagara`) "User.Spraying" true)
    (else
      (`NiagaraComponent.SetVariableBool` (`self.Niagara`) "User.Spraying" false))))

(fn `UserConstructionScript`)
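; Blueprint with five colour trigger boxes (red, green, blue, yellow and random) that reports a selection to the player's VR pawn.
; Each box's begin-overlap event casts player pawn 0 to vrPawn, calls that pawn's matching function and prints a debug message.
; The overlapping actor is never checked, so any overlap fires the selection on the player's pawn.
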(event `self.RedBox.OnComponentBeginOverlap`
  (params (OverlappedComponent :type "PrimitiveComponent Object Reference") (OtherActor :type "Actor Object Reference") (OtherComp :type "PrimitiveComponent Object Reference") (OtherBodyIndex :type Integer) (bFromSweep :type Boolean) (SweepResult :type "HitResult Structure (by ref)"))
  (bind _asvr_pawn (cast `/Game/SprayCan/Blueprints/vrPawn` (`GameplayStatics.GetPlayerPawn` 0))
    (:`then`
      (`/Game/SprayCan/Blueprints/vrPawn.RedBox` _asvr_pawn)
      (`KismetSystemLibrary.PrintString` "RedBox Selected"))
    (:`CastFailed`
      (`KismetSystemLibrary.PrintString` "...why"))))

(event `self.GreenBox.OnComponentBeginOverlap`
  (params (OverlappedComponent :type "PrimitiveComponent Object Reference") (OtherActor :type "Actor Object Reference") (OtherComp :type "PrimitiveComponent Object Reference") (OtherBodyIndex :type Integer) (bFromSweep :type Boolean) (SweepResult :type "HitResult Structure (by ref)"))
  (bind _asvr_pawn (cast `/Game/SprayCan/Blueprints/vrPawn` (`GameplayStatics.GetPlayerPawn` 0)))
  (`/Game/SprayCan/Blueprints/vrPawn.GreenBox` _asvr_pawn)
  (`KismetSystemLibrary.PrintString` "GreenBox Selected"))

(event `self.BlueBox.OnComponentBeginOverlap`
  (params (OverlappedComponent :type "PrimitiveComponent Object Reference") (OtherActor :type "Actor Object Reference") (OtherComp :type "PrimitiveComponent Object Reference") (OtherBodyIndex :type Integer) (bFromSweep :type Boolean) (SweepResult :type "HitResult Structure (by ref)"))
  (bind _asvr_pawn (cast `/Game/SprayCan/Blueprints/vrPawn` (`GameplayStatics.GetPlayerPawn` 0)))
  (`/Game/SprayCan/Blueprints/vrPawn.BlueBox` _asvr_pawn)
  (`KismetSystemLibrary.PrintString` "BlueBox Selected"))

(event `self.YellowBox.OnComponentBeginOverlap`
  (params (OverlappedComponent :type "PrimitiveComponent Object Reference") (OtherActor :type "Actor Object Reference") (OtherComp :type "PrimitiveComponent Object Reference") (OtherBodyIndex :type Integer) (bFromSweep :type Boolean) (SweepResult :type "HitResult Structure (by ref)"))
  (bind _asvr_pawn (cast `/Game/SprayCan/Blueprints/vrPawn` (`GameplayStatics.GetPlayerPawn` 0)))
  (`/Game/SprayCan/Blueprints/vrPawn.YellowBox` _asvr_pawn)
  (`KismetSystemLibrary.PrintString` "YellowBox Selected"))

(event `self.RandomBox.OnComponentBeginOverlap`
  (params (OverlappedComponent :type "PrimitiveComponent Object Reference") (OtherActor :type "Actor Object Reference") (OtherComp :type "PrimitiveComponent Object Reference") (OtherBodyIndex :type Integer) (bFromSweep :type Boolean) (SweepResult :type "HitResult Structure (by ref)"))
  (bind _asvr_pawn (cast `/Game/SprayCan/Blueprints/vrPawn` (`GameplayStatics.GetPlayerPawn` 0)))
  (`/Game/SprayCan/Blueprints/vrPawn.RandomBox` _asvr_pawn)
  (`KismetSystemLibrary.PrintString` "RandomBox Selected"))

(fn `UserConstructionScript`)